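; Fist weapon attachment that places punch and kick collisions and particle effects on its owner for unarmed combat.
; On BeginPlay it attaches each collision to the socket matching that component's object name.
; The same loop attaches four left and right punch and kick particles to fixed Fist sockets and hides them.
; Equip and unequip events toggle only the particles' visibility.
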(event `self.ReceiveBeginPlay`
  (for _array_element (`self.Collisions`)
    (`self.AttachToScene` _array_element (`KismetStringLibrary.Conv_StringToName` (`KismetSystemLibrary.GetObjectName` _array_element)))
    (`|ExecutionSequence`
      (:`then_0`
        (`self.AttachToScene` (`self.LP_Particle`) "Fist_LeftPunch")
        (`self.AttachToScene` (`self.RP_Particle`) "Fist_RightPunch"))
      (:`then_1`
        (`self.AttachToScene` (`self.LK_Particle`) "Fist_LeftKick")
        (`self.AttachToScene` (`self.RK_Particle`) "Fist_RightKick"))
      (:`then_2`
        (`SceneComponent.SetVisibility` (`self.LP_Particle`) false false)
        (`SceneComponent.SetVisibility` (`self.RP_Particle`) false false)
        (`SceneComponent.SetVisibility` (`self.LK_Particle`) false false)
        (`SceneComponent.SetVisibility` (`self.RK_Particle`) false false)))))

(event `self.OnEquip`
  (`SceneComponent.SetVisibility` (`self.LP_Particle`) true false)
  (`SceneComponent.SetVisibility` (`self.RP_Particle`) true false)
  (`SceneComponent.SetVisibility` (`self.LK_Particle`) true false)
  (`SceneComponent.SetVisibility` (`self.RK_Particle`) true false))

(event `self.OnUnequip`
  (`SceneComponent.SetVisibility` (`self.LP_Particle`) false false)
  (`SceneComponent.SetVisibility` (`self.RP_Particle`) false false)
  (`SceneComponent.SetVisibility` (`self.LK_Particle`) false false)
  (`SceneComponent.SetVisibility` (`self.RK_Particle`) false false))

(fn `UserConstructionScript`)